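; BP_SubscriptionHandler is a GraphQL subscription handler that reports connection and message events as printed debug text.
; It overrides the parent's callbacks for connection, start acknowledgement, data, completion, missed keep-alives, errors and socket closure.
; Each override calls the parent implementation, then prints the event name along with any arguments, such as message ID, payload, errors or close status.
; It adds no other logic.
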(event `self.OnConnected`
  (`parent.OnConnected`)
  (`KismetSystemLibrary.PrintString` null "OnConnected"))

(event `self.OnReceiveCompleteMessage`
  (params (id :type String))
  (`parent.OnReceiveCompleteMessage` id)
  (`KismetSystemLibrary.PrintText` null (`|FormatText` "onReceiveCompleteMessage: Id: {0}" id)))

(event `self.OnReceiveDataMessage`
  (params (id :type String) (data :type String))
  (`parent.OnReceiveDataMessage` id data)
  (`KismetSystemLibrary.PrintText` null (`|FormatText` "onReceiveDataMessage: Id: {0}, Data: {1}" id data)))

(event `self.OnReceiveStartACKMessage`
  (params (id :type String))
  (`parent.OnReceiveStartACKMessage` id)
  (`KismetSystemLibrary.PrintText` null (`|FormatText` "onReceiveStartACKMessage: Id: {0}" id)))

(event `self.OnConnectionError`
  (params (errors :type String))
  (`parent.OnConnectionError` errors)
  (`KismetSystemLibrary.PrintText` null (`|FormatText` "OnConnectionError: Errors: {0}" errors)))

(event `self.OnKeepAliveMessageMissed`
  (`parent.OnKeepAliveMessageMissed`)
  (`KismetSystemLibrary.PrintString` null "OnKeepAliveMessageMissed"))

(event `self.OnGraphQLConnectionError`
  (params (errors :type String))
  (`parent.OnGraphQLConnectionError` errors)
  (`KismetSystemLibrary.PrintText` null (`|FormatText` "OnGraphQLConnectionError: Errors: {0}" errors)))

(event `self.OnGraphQLError`
  (params (id :type String) (errors :type String))
  (`parent.OnGraphQLError` id errors)
  (`KismetSystemLibrary.PrintText` null (`|FormatText` "OnGraphQLError: Id: {0}, Errors: {1}" id errors)))

(event `self.OnClosed`
  (params (StatusCode :type Integer) (Reason :type String) (bWasClean :type Boolean))
  (`parent.OnClosed` StatusCode Reason bWasClean)
  (`KismetSystemLibrary.PrintText` null (`|FormatText` "OnClosed: StatusCode: {0}, Reason: {1}, WasClean: {2}" StatusCode Reason bWasClean)))